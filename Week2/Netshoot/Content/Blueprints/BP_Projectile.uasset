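; BP_Projectile is a bullet that resolves its impact on hit, playing a pitch-randomized sound and then destroying itself.
; Hat-tagged components on Characters are knocked off with physics, reduced bullet velocity, random spin and a drop sound, without damage.
; Other Character hits deal effectively fixed damage despite the random-range node, and BP_Ball takes huge damage with a debug print.
; All non-hat hits spawn a hit particle effect.
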(event Collision|EventHit
  (params (MyComp :type Primitive%20Component%20Object%20Reference) (Other :type Actor%20Object%20Reference) (OtherComp :type Primitive%20Component%20Object%20Reference) (bSelfMoved :type Boolean) (HitLocation :type Vector :default "0, 0, 0") (HitNormal :type Vector :default "0, 0, 0") (NormalImpulse :type Vector :default "0, 0, 0") (Hit :type Hit%20Result%20Structure%20%28by%20ref%29))
  (Variables|Default|SetOther Other)
  (Variables|Default|SetOther%20Comp OtherComp)
  (Variables|Default|SetHit%20Location HitLocation)
  ;[0 1 0] BulletHitSound
  (Audio|PlaySoundatLocation "/Game/Sounds/SoundCue_Attentuated.SoundCue_Attentuated" (Variables|Default|GetHit%20Location) "0, 0, 0" (Variables|Default|GetVolumeMultiplier) (Math|Random|RandomFloatinRange 0.8 1.2) 0.0 0 0 0)
  (Utilities|Casting|CastToCharacter (Variables|Default|GetOther)
    (:then
      (if (Components|ComponentHasTag (Variables|Default|GetOther%20Comp) "Hat")
        ;[1 1 1] Hit Hat
        (Actor|DestroyActor)
        (Physics|SetSimulatePhysics (Variables|Default|GetOther%20Comp) true)
        (Physics|SetPhysicsLinearVelocity (Variables|Default|GetOther%20Comp) (/ (Variables|/Script/Engine.MovementComponent|GetVelocity (Variables|Default|GetProjectileMovement)) 3.0) false "None")
        (Class|PrimitiveComponent|SetPhysicsAngularVelocityinDegrees (Variables|Default|GetOther%20Comp) (Math|Vector|MakeVector (Math|Random|RandomFloatinRange -7.2e+02 7.2e+02) (Math|Random|RandomFloatinRange -7.2e+02 7.2e+02) (Math|Random|RandomFloatinRange -7.2e+02 7.2e+02)) false "None")
        ;[0 1 0] HatDropSound
        (Audio|PlaySoundatLocation "/Game/Sounds/Randomize_01.Randomize_01" (Variables|Default|GetHit%20Location) "0, 0, 0" (* (Variables|Default|GetVolumeMultiplier) 0.25) 1.0 0.0 0 0 0)
        (else
          ;[1 1 1] Hit Character
          (Game|Damage|ApplyDamage (Variables|Default|GetOther) (Math|Random|RandomFloatinRange 1.1e+02 1.1e+02) (Game|GetInstigatorController) self)
          ;[1 1 1] BulletDie
          (Actor|DestroyActor :!label _label)
          (Effects|SpawnEmitteratLocation "/Game/Effects/P_Hit.P_Hit" (Variables|Default|GetHit%20Location)))))
    (:CastFailed
      (Utilities|Casting|CastToBP_Ball (Variables|Default|GetOther)
        (:then
          ;[1 1 1] Hit Ball
          (Game|Damage|ApplyDamage (Variables|Default|GetOther) 10086.0 (Game|GetInstigatorController) self)
          (Development|PrintString "hitball")
          (goto _label))
        (:CastFailed
          (goto _label))))))

(fn ConstructionScript)